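; BP_TEST_Wurm2 is a test worm actor that moves along grid points in a back-and-forth, row-descending pattern.
; Tick advances one of two alphas by Speed to lerp its location, either along the row (CWCCW) or down to the next row.
; SetDownLoc stores the row alpha, flips Direction and interpolates a target between below-row points.
; GoingDownTimerDEV fakes the drop trigger from game time, roughly every five seconds.
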(event `self.ReceiveTick`
  (params (DeltaSeconds :type "Float (single-precision)"))
  (bind _nextgridpoint (`self.NextGridpoint`))
  (bind _lastgridpoint (`self.LastGridpoint`))
  (bind _returnvalue (+ (`self.AlphaCWCCW`) 0.1))
  (if (`self.GoingDown`)
    ;[1 1 1] Next Row (Down)
    ;;[1 1 1] Alpha
    (if (> (`self.AlphaDown`) (- 1.0 (`self.Speed`)))
      (set `self.AlphaDown` 0.0)
      ;[1 1 1] End Next Row (down)
      (if (> (`self.direction`) 0)
        (set `self.ComeFromLoc` _lastgridpoint)
        (set `self.GoingToLoc` _nextgridpoint)
        (set `self.AlphaCWCCW` _returnvalue)
        (set `self.GoingDown` false)
        (else
          (set `self.ComeFromLoc` _lastgridpoint)
          (set `self.GoingToLoc` _nextgridpoint)
          (set `self.AlphaCWCCW` _returnvalue)
          (set `self.GoingDown` false)))
      (else
        (bind _output_get (set `self.AlphaDown` (+ (`self.AlphaDown`) (`self.Speed`))))
        ;;[1 1 1] Move
        (`self.K2_SetActorLocation` (`KismetMathLibrary.VLerp` (`self.ComeFromLoc`) (`self.GoingToLoc`) _output_get))))
    (else
      ;[1 1 1] CWCCW
      ;;[1 1 1] Alpha
      (if (> (`self.AlphaCWCCW`) (- 1.0 (`self.Speed`)))
        (set `self.AlphaCWCCW` 0.0)
        ;[1 1 1] End CWCCW
        (set `self.ComeFromLoc` (`self.LastGridpoint`))
        (set `self.GoingToLoc` (`self.NextGridpoint`))
        (else
          (bind _output_get_2 (set `self.AlphaCWCCW` (+ (`self.AlphaCWCCW`) (`self.Speed`))))
          ;;[1 1 1] Move
          (`self.K2_SetActorLocation` (`KismetMathLibrary.VLerp` (`self.ComeFromLoc`) (`self.GoingToLoc`) _output_get_2)))))))

(event `SetDownLoc`
  ;[1 1 1] Set Down Parameters
  (set `self.CollideAlpha` (`self.AlphaCWCCW`)) ; store alpha
  (set `self.AlphaDown` 0.0)
  (set `self.direction` (* (`self.direction`) -1))
  (set `self.ComeFromLoc` (`self.K2_GetActorLocation`))
  (if (> (`self.direction`) 0)
    (set `self.GoingToLoc` (`KismetMathLibrary.VLerp` (`self.BelowPlus`) (`self.BelowLast`) (`self.CollideAlpha`)))
    (else
      (set `self.GoingToLoc` (`KismetMathLibrary.VLerp` (`self.BelowMin`) (`self.BelowLast`) (`self.CollideAlpha`))))))

(fn `GoingDownTimerDEV`
  (if (>= (mod (`KismetSystemLibrary.GetGameTimeInSeconds`) 5.0) 4.98)
    (set `self.GoingDown` true))
  (return))

(fn `UserConstructionScript`)