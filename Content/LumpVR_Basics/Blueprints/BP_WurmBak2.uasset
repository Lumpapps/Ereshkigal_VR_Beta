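; One segment of a Centipede-style wurm enemy in the VR shooter, circling the arena wall along horizontal gridlines.
; Segments spawn as a chain; the leader records positions in a ring buffer, which followers read at offsets.
; The leader moves by timeline and wall traces, dropping a gridline and reversing at obstacles.
; A bullet hit turns the segment into an obstacle and promotes the one behind to leader.
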(event `SpawnFollowurm`
  (bind _returnvalue (`self.K2_GetActorRotation`))
  ;[1 1 1] Spawn Follower
  (bind _asvr_shooter_game_mode (cast `/Game/LumpVR_Basics/Blueprints/VR_ShooterGameMode` (`GameplayStatics.GetGameMode`)))
  (`/Engine/EditorBlueprintResources/StandardMacros.IncrementInt` (`/Game/LumpVR_Basics/Blueprints/VR_ShooterGameMode.Wurm1NumberSpawned` _asvr_shooter_game_mode)
    (:`  `
      (bind _returnvalue_2 (`|SpawnActorFromClass` "BP_WurmBak2_C" (`KismetMathLibrary.MakeTransform` (+ (`self.K2_GetActorLocation`) (`KismetMathLibrary.MakeVector` (- (.x (`KismetMathLibrary.GetForwardVector` _returnvalue)) (* (`.SphereRadius` (`KismetSystemLibrary.GetComponentBounds` (`self.wurmpart`))) 1.0)) (.y (`KismetMathLibrary.GetForwardVector` _returnvalue)) (.z (`KismetMathLibrary.GetForwardVector` _returnvalue)))) _returnvalue) "AlwaysSpawn" "OverrideRootScale" null null))
      (set `self.WurmBehind` _returnvalue_2)
      ;[1 1 1] Tell wurms who is there initial leader, wurm in front and wurm behind
      (if (`self.Leader`)
        (set `/Game/LumpVR_Basics/Blueprints/BP_WurmBak2.MyLead` self _returnvalue_2)
        (else
          (`KismetSystemLibrary.Delay` 0.1)
          (bind _asbp_wurm (cast `/Game/LumpVR_Basics/Blueprints/BP_WurmBak2` (`self.MyLead`)))
          (set `/Game/LumpVR_Basics/Blueprints/BP_WurmBak2.MyLead` _asbp_wurm _returnvalue_2)
          (set `/Game/LumpVR_Basics/Blueprints/BP_WurmBak2.WurmFront` self _returnvalue_2))))))

(event `self.ReceiveBeginPlay`
  (bind (_returnvalue_x _returnvalue_y) (`KismetMathLibrary.BreakVector` (`self.K2_GetActorLocation`)))
  (bind _asvr_shooter_game_mode (cast `/Game/LumpVR_Basics/Blueprints/VR_ShooterGameMode` (`GameplayStatics.GetGameMode`)))
  (set `self.Speed` (`/Game/LumpVR_Basics/Blueprints/VR_ShooterGameMode.WurmSpeed` _asvr_shooter_game_mode))
  (set `self.ArenaHeight` (* 2 (.z (`.BoxExtent` (`self.GetActorBounds` (`/Game/LumpVR_Basics/Blueprints/VR_ShooterGameMode.Arena` _asvr_shooter_game_mode) false false)))))
  ;[1 1 1] Set actor to first gridline
  (bind _asvr_shooter_game_mode_2 (cast `/Game/LumpVR_Basics/Blueprints/VR_ShooterGameMode` (`GameplayStatics.GetGameMode`)))
  (bind _output (`|GetArrayItem` (`/Game/LumpVR_Basics/Blueprints/VR_ShooterGameMode.GridlinesHorizontal` _asvr_shooter_game_mode_2) (`self.GridlineIndex`)))
  (bind _position_new (`self.GetActorArenaPos` (`KismetMathLibrary.MakeVector` _returnvalue_x _returnvalue_y _output))) ; Set ON instead of IN arena
  (bind _x (.x _position_new))
  (bind _y (.y _position_new))
  (`self.K2_SetActorLocation` (`KismetMathLibrary.MakeVector` _x _y _output)) ; set actor to first gridline
  (bind _output_get (set `self.CurrentLoc` (`KismetMathLibrary.MakeVector` _x _y _output)))
  (`self.K2_SetActorRotation` (`KismetMathLibrary.ComposeRotators` (`KismetMathLibrary.FindLookAtRotation` (.location (`SceneComponent.K2_GetComponentToWorld` (`self.wurmpart`))) (`KismetMathLibrary.MakeVector` 0.0 0.0 (.z _output_get))) (`KismetMathLibrary.MakeRotator` 0.0 0.0 (* -90 (`self.Direction`)))))
  (bind _asvr_shooter_game_mode_3 (cast `/Game/LumpVR_Basics/Blueprints/VR_ShooterGameMode` (`GameplayStatics.GetGameMode`)))
  (bind _output_get_2 (set `self.Wurmnumber` (`/Game/LumpVR_Basics/Blueprints/VR_ShooterGameMode.Wurm1NumberSpawned` _asvr_shooter_game_mode_3)))
  (if (== _output_get_2 0)
    (set `self.Leader` true)
    (set `self.MyLead` self) ; For when killed See end overlap
    (bind _asvr_shooter_game_mode_4 (cast `/Game/LumpVR_Basics/Blueprints/VR_ShooterGameMode` (`GameplayStatics.GetGameMode`)))
    (if (== (`/Game/LumpVR_Basics/Blueprints/VR_ShooterGameMode.Wurm1NumberSpawned` _asvr_shooter_game_mode_4) 0)
      (`self.SpawnFollowurm`)
      (bind _asvr_shooter_game_mode_5 (cast `/Game/LumpVR_Basics/Blueprints/VR_ShooterGameMode` (`GameplayStatics.GetGameMode`)))
      (if (== (`/Game/LumpVR_Basics/Blueprints/VR_ShooterGameMode.Wurm1NumberSpawned` _asvr_shooter_game_mode_5) (- (`/Game/LumpVR_Basics/Blueprints/VR_ShooterGameMode.Wurm1Length` _asvr_shooter_game_mode_5) 1))
        ;[1 1 1] Create empty positions
        (for _ (range 1000)
          (`KismetArrayLibrary.Array_Add` (`self.Positions`))
          (`self.CWCCW`))))
    (else
      (set `self.Leader` false)
      (bind _asvr_shooter_game_mode_6 (cast `/Game/LumpVR_Basics/Blueprints/VR_ShooterGameMode` (`GameplayStatics.GetGameMode`)))
      (if (< (`self.Wurmnumber`) (- (`/Game/LumpVR_Basics/Blueprints/VR_ShooterGameMode.Wurm1Length` _asvr_shooter_game_mode_6) 1))
        (`self.SpawnFollowurm`)))))

(event `CWCCW`
  (bind _speed (`self.Speed`))
  (bind (_currentloc_x _currentloc_y _currentloc_z) (`KismetMathLibrary.BreakVector` (`self.CurrentLoc`)))
  ;[1 1 1] Sideways Clockwise Counterclockwise
  (bind (_direction _position) (`Timeline|TimelineEndles` :!via `PlayFromStart` :!label _label)
    (:`Update`
      (if (< _position (* (`KismetMathLibrary.GetPI`) (* (/ 1.0 _speed) 2.0)))
        (bind _returnvalue (+ (`KismetMathLibrary.Atan2` _currentloc_y _currentloc_x) (* _position (* _speed (`self.Direction`)))))
        (bind _outhit (`KismetSystemLibrary.LineTraceSingle` (`KismetMathLibrary.MakeVector` 0.0 0.0 _currentloc_z) (`KismetMathLibrary.MakeVector` (* (`KismetMathLibrary.Cos` _returnvalue) 5000.0) (* (`KismetMathLibrary.Sin` _returnvalue) 5000.0) _currentloc_z) "TraceTypeQuery1"))
        (bind (_bblockinghit _binitialoverlap _time _distance _location _impactpoint _normal _impactnormal _physmat _hitactor) (`GameplayStatics.BreakHitResult` _outhit))
        (if (== (`GameplayStatics.GetObjectClass` _hitactor) "/Game/LumpVR_Basics/Blueprints/BP_Arena01.BP_Arena01_C")
          (bind _position_new (`self.GetActorArenaPos` _location))
          (`self.K2_SetActorTransform` (`KismetMathLibrary.MakeTransform` _position_new (`KismetMathLibrary.ComposeRotators` (`KismetMathLibrary.FindLookAtRotation` (.location (`SceneComponent.K2_GetComponentToWorld` (`self.wurmpart`))) (`KismetMathLibrary.MakeVector` 0.0 0.0 _currentloc_z)) (`KismetMathLibrary.MakeRotator` 0.0 0.0 (* -90 (`self.Direction`)))) (.scale (`SceneComponent.K2_GetComponentToWorld` (`self.wurmpart`))))))
        (else
          (goto _label :!via `PlayFromStart`))))))

(event `StopCWCCW`
  ;[1 1 1] Sideways Clockwise Counterclockwise
  (goto _label :!via `Stop`))

(event `DDown`
  ;[1 1 1] Down
  ;;[1 1 1] My Lead to behind
  (bind _asbp_wurm (cast `/Game/LumpVR_Basics/Blueprints/BP_WurmBak2` (`self.WurmBehind`)))
  (bind _asbp_wurm_2 (cast `/Game/LumpVR_Basics/Blueprints/BP_WurmBak2` (`self.MyLead`)))
  (set `/Game/LumpVR_Basics/Blueprints/BP_WurmBak2.MyLead` _asbp_wurm_2 _asbp_wurm)
  (bind _output_get (set `self.CurrentLoc` (`self.K2_GetActorLocation`)))
  (bind _asvr_shooter_game_mode (cast `/Game/LumpVR_Basics/Blueprints/VR_ShooterGameMode` (`GameplayStatics.GetGameMode`)))
  (bind _output (`|GetArrayItem` (`/Game/LumpVR_Basics/Blueprints/VR_ShooterGameMode.GridlinesHorizontal` _asvr_shooter_game_mode) (`KismetMathLibrary.Clamp` (+ 1 (`self.GridlineIndex`)) 0 (`KismetArrayLibrary.Array_LastIndex` (`/Game/LumpVR_Basics/Blueprints/VR_ShooterGameMode.GridlinesHorizontal` _asvr_shooter_game_mode)))))
  (bind _outhit (`KismetSystemLibrary.LineTraceSingle` (`KismetMathLibrary.MakeVector` 0.0 0.0 (.z _output_get)) (`KismetMathLibrary.MakeVector` (* (.x _output_get) 2.0) (* (.y _output_get) 2.0) _output) "TraceTypeQuery1"))
  (bind (_bblockinghit _binitialoverlap _time _distance _location _impactpoint _normal _impactnormal _physmat _hitactor) (`GameplayStatics.BreakHitResult` _outhit))
  (if (== (`GameplayStatics.GetObjectClass` _hitactor) "/Game/LumpVR_Basics/Blueprints/BP_Arena01.BP_Arena01_C")
    (bind _position_new (`self.GetActorArenaPos` _location))
    (bind (_direction _alpha) (`Timeline|LerpAlpha` :!via `PlayFromStart`)
      (:`Update`
        ;;[1 1 1] Comment
        (`self.K2_SetActorTransform` (`KismetMathLibrary.MakeTransform` (`KismetMathLibrary.VLerp` (`self.CurrentLoc`) _position_new _alpha) (`KismetMathLibrary.ComposeRotators` (`KismetMathLibrary.FindLookAtRotation` (.location (`self.GetTransform`)) (`KismetMathLibrary.MakeVector` 0.0 0.0 _output)) (`KismetMathLibrary.MakeRotator` 0.0 0.0 (* -90 (`self.Direction`)))) (.scale (`self.GetTransform`)))))
      (:`Finished`
        ;;[1 1 1] Change direction and move
        (set `self.CurrentLoc` (`self.K2_GetActorLocation`))
        (set `self.Direction` (* (`self.Direction`) -1.0))
        (bind _asvr_shooter_game_mode_2 (cast `/Game/LumpVR_Basics/Blueprints/VR_ShooterGameMode` (`GameplayStatics.GetGameMode`)))
        (set `self.GridlineIndex` (`KismetMathLibrary.Clamp` (+ (`self.GridlineIndex`) 1) 0 (`KismetArrayLibrary.Array_LastIndex` (`/Game/LumpVR_Basics/Blueprints/VR_ShooterGameMode.GridlinesHorizontal` _asvr_shooter_game_mode_2))))
        (`self.CWCCW`)))))

(event `self.ReceiveTick`
  (params (DeltaSeconds :type "Float (single-precision)"))
  (bind _wurmpart (`self.wurmpart`))
  (bind _z (.z (`self.K2_GetActorLocation`)))
  (if (`self.Leader`)
    ;[1 1 1] ChangetoLeadorFollower
    (`PrimitiveComponent.SetMaterial` _wurmpart 0 "/Game/VirtualReality/Materials/M_ArcEndpoint.M_ArcEndpoint")
    (`StaticMeshComponent.SetStaticMesh` _wurmpart "/Game/Geometry/Meshes/1M_Cube.1M_Cube")
    ;[1 1 1] Set locations - positions array is pre-filled in event start
    (`KismetArrayLibrary.Array_Set` (`self.Positions`) (`self.PositionIndexCount`) (`self.K2_GetActorLocation`))
    (set `self.PositionIndexCount` (mod (+ (`self.PositionIndexCount`) 1) 1000))
    (else
      (`PrimitiveComponent.SetMaterial` _wurmpart 0 "/Game/LumpVR_Basics/VFX/MICs/MI_VolumeFlame.MI_VolumeFlame")
      (`StaticMeshComponent.SetStaticMesh` _wurmpart "/Engine/BasicShapes/Sphere.Sphere")
      ;[1 1 1] Get location
      (bind _asvr_shooter_game_mode (cast `/Game/LumpVR_Basics/Blueprints/VR_ShooterGameMode` (`GameplayStatics.GetGameMode`)))
      (bind _asbp_wurm (cast `/Game/LumpVR_Basics/Blueprints/BP_WurmBak2` (`self.MyLead`)))
      (bind _returnvalue (- (`/Game/LumpVR_Basics/Blueprints/BP_WurmBak2.PositionIndexCount` _asbp_wurm) (* (`self.Wurmnumber`) (+ (`/Game/LumpVR_Basics/Blueprints/VR_ShooterGameMode.WurmDistance` _asvr_shooter_game_mode) (`KismetMathLibrary.FTrunc` (* (/ (`self.ArenaHeight`) (`KismetMathLibrary.VSize` (- (`KismetMathLibrary.MakeVector` (.x (`self.K2_GetActorLocation`)) (.y (`self.K2_GetActorLocation`)) _z) (`KismetMathLibrary.MakeVector` (.x (`KismetMathLibrary.MakeVector` 0.0 0.0 _z)) (.y (`KismetMathLibrary.MakeVector` 0.0 0.0 _z)) (.z (`KismetMathLibrary.MakeVector` 0.0 0.0 _z)))))) 5.0))))))
      (if (< _returnvalue 0)
        (set `self.PosIndexPositive` (+ _returnvalue 1000))
        (else
          (set `self.PosIndexPositive` _returnvalue)))
      (`self.K2_SetActorTransform` (`KismetMathLibrary.MakeTransform` (`|GetArrayItem` (`/Game/LumpVR_Basics/Blueprints/BP_WurmBak2.Positions` _asbp_wurm) (`self.PosIndexPositive`)) (`self.K2_GetActorRotation` _asbp_wurm))))))

(event `self.InFrontCollision.OnComponentBeginOverlap`
  (params (OverlappedComponent :type "PrimitiveComponent Object Reference") (OtherActor :type "Actor Object Reference") (OtherComp :type "PrimitiveComponent Object Reference") (OtherBodyIndex :type Integer) (bFromSweep :type Boolean) (SweepResult :type "HitResult Structure (by ref)")))

(event `self.InFrontCollision.OnComponentEndOverlap`
  (params (OverlappedComponent :type "PrimitiveComponent Object Reference") (OtherActor :type "Actor Object Reference") (OtherComp :type "PrimitiveComponent Object Reference") (OtherBodyIndex :type Integer)))

(event `self.Sphere.OnComponentBeginOverlap`
  (params (OverlappedComponent :type "PrimitiveComponent Object Reference") (OtherActor :type "Actor Object Reference") (OtherComp :type "PrimitiveComponent Object Reference") (OtherBodyIndex :type Integer) (bFromSweep :type Boolean) (SweepResult :type "HitResult Structure (by ref)"))
  (bind (_returnvalue_roll _returnvalue_pitch _returnvalue_yaw) (`KismetMathLibrary.BreakRotator` (`KismetMathLibrary.RandomRotator` false)))
  (bind _returnvalue (`self.K2_GetActorLocation`))
  (bind _returnvalue_2 (`GameplayStatics.GetObjectClass` OtherActor))
  (if (== _returnvalue_2 "/Game/LumpVR_Basics/Blueprints/BP_BulletProjectile.BP_BulletProjectile_C")
    ;[1 1 1] Tell the one behind (if valid) it is the leader
    (`self.WurmBehind`
      (:`then`
        (bind _asbp_wurm (cast `/Game/LumpVR_Basics/Blueprints/BP_WurmBak2` (`self.WurmBehind`)))
        (`self.DDown` _asbp_wurm)
        (set `/Game/LumpVR_Basics/Blueprints/BP_WurmBak2.Leader` true _asbp_wurm)
        (set `/Game/LumpVR_Basics/Blueprints/BP_WurmBak2.MyLead` _asbp_wurm _asbp_wurm) ; Set MyLead to itself
      )
      (:`else`
        _))
    ;[1 1 1] Hit Something
    (`|SpawnActorFromClass` "/Game/LumpVR_Basics/Blueprints/BP_Obstacle.BP_Obstacle_C" (`KismetMathLibrary.MakeTransform` _returnvalue (`KismetMathLibrary.MakeRotator` (`KismetMathLibrary.FClamp` _returnvalue_roll 0.0 10.0) (`KismetMathLibrary.FClamp` _returnvalue_pitch 0.0 10.0) _returnvalue_yaw)) "Undefined" "OverrideRootScale" null null)
    (`GameplayStatics.SpawnSoundAtLocation` "/Game/StarterContent/Audio/Explosion01.Explosion01" _returnvalue (struct) 1.0 1.0 0.0 null null)
    (`self.K2_DestroyActor`)
    (elif (`self.Leader`)
      (if (== _returnvalue_2 "/Game/LumpVR_Basics/Blueprints/BP_Obstacle.BP_Obstacle_C")
        (if (not (`KismetArrayLibrary.Array_Contains` (`self.HitObstacles`) OtherActor))
          ;[1 1 1] Make list of hit obtacles so they don't trigger twice
          (`KismetArrayLibrary.Array_Add` (`self.HitObstacles`) OtherActor)
          (`self.StopCWCCW`)
          (`self.DDown`))))))

(fn `Deform`
  (params (ThisPart :type "StaticMeshComponent Object Reference") (ClosePart :type "Actor Object Reference") (Distance :type "Float (double-precision)"))
  (if (== (`GameplayStatics.GetObjectClass` ClosePart) (`GameplayStatics.GetObjectClass` self))
    (bind _returnvalue (`PrimitiveComponent.CreateDynamicMaterialInstance` ThisPart 0 null "NextInLineLoc"))
    (if (> Distance 0.0)
      (`MaterialInstanceDynamic.SetVectorParameterValue` _returnvalue "NextInLineLoc" (`KismetMathLibrary.Conv_VectorToLinearColor` (`self.K2_GetActorLocation` ClosePart)))
      (else
        (`MaterialInstanceDynamic.SetVectorParameterValue` _returnvalue "NextInLineLoc" (struct :`A` 1.0))))
    (else
      (bind _returnvalue_2 (`PrimitiveComponent.CreateDynamicMaterialInstance` ThisPart 0 null "NextInLineLoc"))
      (`MaterialInstanceDynamic.SetVectorParameterValue` :`self` _returnvalue_2 :`ParameterName` "NextInLineLoc"))))

(fn `GetActorArenaPos`
  (params (`position old` :type "Vector Structure"))
  (returns (`position new` :type "Vector Structure"))
  (bind _x (.x `position old`))
  (bind _y (.y `position old`))
  (bind _z (.z `position old`))
  (bind _returnvalue (`KismetMathLibrary.Atan2` _y _x))
  (bind (_origin _boxextent _sphereradius) (`KismetSystemLibrary.GetComponentBounds` (`self.Sphere`)))
  (bind _outhit (`KismetSystemLibrary.LineTraceSingle` (`KismetMathLibrary.MakeVector` 0.0 0.0 _z) (`KismetMathLibrary.MakeVector` (* _x 5000.0) (* _y 5000.0) _z) "TraceTypeQuery1"))
  (bind (_bblockinghit _binitialoverlap _time _distance _location _impactpoint _normal _impactnormal _physmat _hitactor) (`GameplayStatics.BreakHitResult` _outhit))
  (if (== (`GameplayStatics.GetObjectClass` _hitactor) "/Game/LumpVR_Basics/Blueprints/BP_Arena01.BP_Arena01_C")
    (return (`KismetMathLibrary.MakeVector` (- (.x _location) (/ (* _sphereradius (`KismetMathLibrary.DegSin` (- (- 180.0 (`KismetMathLibrary.RadiansToDegrees` _returnvalue)) 90.0))) (`KismetMathLibrary.DegSin` 90.0))) (- (.y _location) (/ (* _sphereradius (`KismetMathLibrary.DegSin` (`KismetMathLibrary.RadiansToDegrees` _returnvalue))) (`KismetMathLibrary.DegSin` 90.0))) (.z _location)))))

(fn `UserConstructionScript`)