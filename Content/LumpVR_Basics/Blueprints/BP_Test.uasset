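; BP_Test is a test actor that passes an integer between overlapping instances of itself, with a lead instance starting at 99.
; On box overlap, a non-lead stores a same-class actor as Frontrunner, increments that actor's IAmVar, copies it and prints debug results.
; Tick keeps copying IAmVar from the overlap event's OtherActor, even for leads.
; End overlap clears Frontrunner.
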(event `self.ReceiveBeginPlay`
  (if (`self.Lead`)
    (set `self.IAmVar` 99)))

(event `self.ReceiveTick`
  (params (DeltaSeconds :type "Float (single-precision)"))
  (bind _asbp_test (cast `/Game/LumpVR_Basics/Blueprints/BP_Test` (stale `self.Box.OnComponentBeginOverlap` OtherActor)))
  (bind _output_get (set `self.IAmVar` (`/Game/LumpVR_Basics/Blueprints/BP_Test.IAmVar` _asbp_test))))

(event `self.Box.OnComponentBeginOverlap`
  (params (OverlappedComponent :type "PrimitiveComponent Object Reference") (OtherActor :type "Actor Object Reference") (OtherComp :type "PrimitiveComponent Object Reference") (OtherBodyIndex :type Integer) (bFromSweep :type Boolean) (SweepResult :type "HitResult Structure (by ref)"))
  (if (not (`self.Lead`))
    (if (== (`GameplayStatics.GetObjectClass` OtherActor) (`GameplayStatics.GetObjectClass` self))
      (set `self.Frontrunner` OtherActor)
      (`KismetSystemLibrary.PrintString` "OtherisSame")
      (else
        (`KismetSystemLibrary.PrintString` "OtherisDifferent")))
    (bind _asbp_test (cast `/Game/LumpVR_Basics/Blueprints/BP_Test` OtherActor))
    (if (`/Game/LumpVR_Basics/Blueprints/BP_Test.Lead` _asbp_test)
      (`KismetSystemLibrary.PrintString` "OtherisLead")
      (else
        (`KismetSystemLibrary.PrintString` "Otherisnolead")))
    (bind _iamvar (`/Game/LumpVR_Basics/Blueprints/BP_Test.IAmVar` _asbp_test))
    (`/Engine/EditorBlueprintResources/StandardMacros.IncrementInt` _iamvar
      (:`  `
        (bind _output_get (set `self.IAmVar` _iamvar))
        (`KismetSystemLibrary.PrintString` (`KismetStringLibrary.Conv_IntToString` _output_get))))))

(event `self.Box.OnComponentEndOverlap`
  (params (OverlappedComponent :type "PrimitiveComponent Object Reference") (OtherActor :type "Actor Object Reference") (OtherComp :type "PrimitiveComponent Object Reference") (OtherBodyIndex :type Integer))
  (bind _output_get (set `self.Frontrunner` null))
  (`KismetSystemLibrary.PrintString` (`KismetSystemLibrary.GetDisplayName` _output_get)))

(fn `UserConstructionScript`)