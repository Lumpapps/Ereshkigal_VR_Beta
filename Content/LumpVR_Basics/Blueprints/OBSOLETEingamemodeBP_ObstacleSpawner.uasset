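; An obsolete obstacle spawner Blueprint that is meant to scatter BP_Obstacle actors over the surface beneath a collision box.
; A 100-plus iteration loop traces downward from random points in the box and spawns at each hit, slightly sunk, rotated by a look-at toward the impact normal.
; Spawns adjust for collisions or are skipped.
; The loop is disconnected and BeginPlay is empty, so nothing spawns as it stands.
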(event `self.ReceiveBeginPlay`)

(fn `UserConstructionScript`)