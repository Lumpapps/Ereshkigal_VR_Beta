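; Player projectile for a VR worm shooter that damages BP_Wurm actors and wurm-hit-spawn obstacles and gates the player's reloading.
; It plays an explosion cue at world origin on spawn.
; Sphere overlaps call BulletHit on worms (Damage variable) or obstacles (fixed amount).
; Those hits, pawn overlaps, or rising above twice the arena's vertical extent all re-enable the pawn's CanLoad and destroy the bullet.
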(event `self.ReceiveBeginPlay`
  (`GameplayStatics.SpawnSoundAtLocation` "/Game/StarterContent/Audio/Explosion_Cue.Explosion_Cue" (0.0 0.0 0.0) (struct) 1.0 1.0 0.0 null null))

(event `self.ReceiveTick`
  (params (DeltaSeconds :type "Float (single-precision)"))
  (bind (_returnvalue_x _returnvalue_y _returnvalue_z) (`KismetMathLibrary.BreakVector` (`self.K2_GetActorLocation`)))
  ;[1 1 1] Reload and Destroy when to high
  (bind _asvr_shooter_game_mode (cast `/Game/LumpVR_Basics/Blueprints/VR_ShooterGameMode` (`GameplayStatics.GetGameMode`)))
  (if (> _returnvalue_z (* 2 (.z (`.BoxExtent` (`self.GetActorBounds` (`/Game/LumpVR_Basics/Blueprints/VR_ShooterGameMode.Arena` _asvr_shooter_game_mode) false false)))))
    (bind _asbp_motion_controller_pawn (cast `/Game/LumpVR_Basics/Blueprints/BP_MotionControllerPawn` (`GameplayStatics.GetPlayerPawn` 0) :!label _label))
    (set `/Game/LumpVR_Basics/Blueprints/BP_MotionControllerPawn.CanLoad` true _asbp_motion_controller_pawn)
    (`self.K2_DestroyActor`)))

(event `self.Sphere.OnComponentBeginOverlap`
  (params (OverlappedComponent :type "PrimitiveComponent Object Reference") (OtherActor :type "Actor Object Reference") (OtherComp :type "PrimitiveComponent Object Reference") (OtherBodyIndex :type Integer) (bFromSweep :type Boolean) (SweepResult :type "HitResult Structure (by ref)"))
  (bind _returnvalue (`GameplayStatics.GetObjectClass` OtherActor))
  (if (`self.IamUsed`)
    _
    (elif (== _returnvalue "/Game/LumpVR_Basics/Blueprints/BP_Wurm.BP_Wurm_C")
      (set `self.IamUsed` true)
      (bind _asbp_wurm (cast `/Game/LumpVR_Basics/Blueprints/BP_Wurm` OtherActor)
        (:`then`
          (`/Game/LumpVR_Basics/Blueprints/BP_Wurm.BulletHit` _asbp_wurm (`self.Damage`))
          (goto _label))
        (:`CastFailed`
          (goto _label)))
      (elif (== _returnvalue "/Game/LumpVR_Basics/Blueprints/BP_Obstacle_WurmhitSpawn.BP_Obstacle_WurmhitSpawn_C")
        (bind _asbp_obstacle_wurmhit_spawn (cast `/Game/LumpVR_Basics/Blueprints/BP_Obstacle_WurmhitSpawn` OtherActor)
          (:`then`
            (`/Game/LumpVR_Basics/Blueprints/BP_Obstacle_WurmhitSpawn.BulletHit` _asbp_obstacle_wurmhit_spawn 25)
            (goto _label))
          (:`CastFailed`
            (goto _label)))
        (elif (== _returnvalue "/Game/LumpVR_Basics/Blueprints/BP_MotionControllerPawn.BP_MotionControllerPawn_C")
          (goto _label))))))

(fn `UserConstructionScript`)