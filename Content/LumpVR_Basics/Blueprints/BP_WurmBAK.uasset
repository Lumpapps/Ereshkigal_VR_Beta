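; One segment of a Centipede-style worm enemy in a VR shooter, apparently a backup of BP_Wurm, whose class it spawns and casts to.
; Segments spawn as a chain; the leader circles the arena wall via line traces, reversing and dropping a gridline on obstacle hits.
; Followers replay the leader's timer-recorded position ring buffer and pass the front segment's location to their material for deformation.
; A killed segment promotes the one behind to leader and leaves an obstacle.
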(event `self.ReceiveBeginPlay`
  (bind (_returnvalue_x _returnvalue_y) (`KismetMathLibrary.BreakVector` (`self.K2_GetActorLocation`)))
  (bind (_currentloc_x _currentloc_y _currentloc_z) (`KismetMathLibrary.BreakVector` (`self.CurrentLoc`)))
  (bind (_currentloc_x_2 _currentloc_y_2) (`KismetMathLibrary.BreakVector` (`self.CurrentLoc`)))
  (bind _returnvalue (+ (* (`/Game/LumpVR_Basics/Blueprints/VR_ShooterGameMode.ArenaHeight` (`self.GamemodeShort`)) 2.0) (.z (`.BoxExtent` (`KismetSystemLibrary.GetComponentBounds` (`self.wurmpart`))))))
  ;[1 1 1] Frequently used variables
  (bind _asvr_shooter_game_mode (cast `/Game/LumpVR_Basics/Blueprints/VR_ShooterGameMode` (`GameplayStatics.GetGameMode`)))
  (bind _output_get (set `self.GamemodeShort` _asvr_shooter_game_mode))
  (set `self.Speed` (`/Game/LumpVR_Basics/Blueprints/VR_ShooterGameMode.WurmSpeed` _output_get))
  ;[1 1 1] Create empty positions array
  (for _ (range (+ (`self.Stored LocationsCount`) 1))
    (`KismetArrayLibrary.Array_Add` (`self.Positions`)))
  ;[1 1 1] Make lead or not, Set MyLead and Spawn Followers
  (if (== (`/Game/LumpVR_Basics/Blueprints/VR_ShooterGameMode.WurmPartNumberSpawned` (`self.GamemodeShort`)) 0)
    (set `self.IAmLeader` true)
    (set `self.MyLead` self) ; For when killed See end overlap
    (`self.SpawnFollowurm`)
    (`self.SetMaterialandMesh`)
    ;[1 1 1] Set at start position
    (`self.K2_SetActorLocation` (`KismetMathLibrary.MakeVector` _returnvalue_x _returnvalue_y _returnvalue))
    ;[1 1 1] Rotation
    (bind _output_get_2 (set `self.CurrentLoc` (`KismetMathLibrary.MakeVector` _returnvalue_x _returnvalue_y _returnvalue)))
    (`self.K2_SetActorRotation` (`KismetMathLibrary.FindLookAtRotation` (`KismetMathLibrary.MakeVector` (.x _output_get_2) (.y _output_get_2) (.z _output_get_2)) (`KismetMathLibrary.MakeVector` 0.0 0.0 (.z _output_get_2))))
    ;[1 1 1] Start storing positions
    (`self.EachXTimer`)
    ;[1 1 1] Move actor to the edge
    (bind _position_new (`self.GetActorArenaPos` (`KismetMathLibrary.MakeVector` _currentloc_x_2 _currentloc_y_2 (`|GetArrayItem` (`/Game/LumpVR_Basics/Blueprints/VR_ShooterGameMode.GridlinesHorizontal` (`self.GamemodeShort`)) (`self.CurrentGridline`))))) ; Set ON instead of IN arena
    (bind (_direction _positionalpha) (`Timeline|WalkToEdge` :!via `PlayFromStart`)
      (:`Update`
        (`self.K2_SetActorLocation` (`KismetMathLibrary.VLerp` (`self.CurrentLoc`) (`KismetMathLibrary.MakeVector` (.x _position_new) (.y _position_new) _currentloc_z) _positionalpha)) ; set actor to first gridline
      )
      (:`Finished`
        (`self.DDown`)
        (set `self.SetupDone` true)))
    (else
      (set `self.IAmLeader` false)
      (if (< (`self.Wurmnumber`) (- (`/Game/LumpVR_Basics/Blueprints/VR_ShooterGameMode.WurmLength` (`self.GamemodeShort`)) 1))
        (`self.SpawnFollowurm`)
        (`self.SetMaterialandMesh`)
        ;;[1 1 1] Start following
        (`self.EachXTimer`)
        (set `self.SetupDone` true)))))

(event `SpawnFollowurm`
  (bind _gamemodeshort (`self.GamemodeShort`))
  ;[1 1 1] Spawn Follower
  (bind _result (`/Engine/EditorBlueprintResources/StandardMacros.IncrementInt` (`/Game/LumpVR_Basics/Blueprints/VR_ShooterGameMode.WurmPartNumberSpawned` _gamemodeshort))
    (:`  `
      (if (< _result (`/Game/LumpVR_Basics/Blueprints/VR_ShooterGameMode.WurmLength` _gamemodeshort))
        (bind _returnvalue (`|SpawnActorFromClass` "/Game/LumpVR_Basics/Blueprints/BP_Wurm.BP_Wurm_C" (`KismetMathLibrary.MakeTransform` (0.0 0.0 -5000.0)) "AlwaysSpawn" "OverrideRootScale" null null))
        ;[1 1 1] Tell wurms who is there initial leader, wurm in front and wurm behind
        (bind _output_get (set `self.WurmBehind` _returnvalue))
        (bind _asbp_wurm (cast `/Game/LumpVR_Basics/Blueprints/BP_Wurm` _output_get))
        (set `/Game/LumpVR_Basics/Blueprints/BP_Wurm.Wurmnumber` _result _asbp_wurm)
        (if (`self.IAmLeader`)
          (set `/Game/LumpVR_Basics/Blueprints/BP_Wurm.MyLead` self _returnvalue)
          (else
            (`KismetSystemLibrary.Delay` 0.1)
            (bind _asbp_wurm_2 (cast `/Game/LumpVR_Basics/Blueprints/BP_Wurm` (`self.MyLead`)))
            (set `/Game/LumpVR_Basics/Blueprints/BP_Wurm.MyLead` _asbp_wurm_2 _returnvalue)
            (set `/Game/LumpVR_Basics/Blueprints/BP_Wurm.WurmFront` self _returnvalue)))))))

(event `DDown`
  (bind _gamemodeshort (`self.GamemodeShort`))
  (bind _output (`|GetArrayItem` (`/Game/LumpVR_Basics/Blueprints/VR_ShooterGameMode.GridlinesHorizontal` _gamemodeshort) (`KismetMathLibrary.Clamp` (+ 1 (`self.CurrentGridline`)) 0 (`KismetArrayLibrary.Array_LastIndex` (`/Game/LumpVR_Basics/Blueprints/VR_ShooterGameMode.GridlinesHorizontal` _gamemodeshort)))))
  ;[1 1 1] Down
  ;[1 1 1] Change direction
  (set `self.Direction` (* (`self.Direction`) -1.0))
  (bind _output_get (set `self.CurrentLoc` (`self.K2_GetActorLocation`)))
  (bind _outhit (`KismetSystemLibrary.LineTraceSingle` (`KismetMathLibrary.MakeVector` 0.0 0.0 (.z _output_get)) (`KismetMathLibrary.MakeVector` (* (.x _output_get) 2.0) (* (.y _output_get) 2.0) _output) "TraceTypeQuery1"))
  (bind (_bblockinghit _binitialoverlap _time _distance _location _impactpoint _normal _impactnormal _physmat _hitactor) (`GameplayStatics.BreakHitResult` _outhit))
  (if (== (`GameplayStatics.GetObjectClass` _hitactor) "/Game/LumpVR_Basics/Blueprints/BP_Arena01.BP_Arena01_C")
    (bind _position_new (`self.GetActorArenaPos` _location))
    (bind (_direction _alpha) (`Timeline|LerpAlpha` :!via `PlayFromStart`)
      (:`Update`
        ;;[1 1 1] Comment
        (`self.K2_SetActorTransform` (`KismetMathLibrary.MakeTransform` (`KismetMathLibrary.VLerp` (`self.CurrentLoc`) _position_new _alpha) (`KismetMathLibrary.ComposeRotators` (`KismetMathLibrary.FindLookAtRotation` (.location (`self.GetTransform`)) (`KismetMathLibrary.MakeVector` 0.0 0.0 _output)) (`KismetMathLibrary.MakeRotator` 0.0 0.0 (* -90 (`self.Direction`)))) (.scale (`self.GetTransform`)))))
      (:`Finished`
        (set `self.CurrentLoc` (`self.K2_GetActorLocation`))
        (set `self.CurrentGridline` (`KismetMathLibrary.Clamp` (+ (`self.CurrentGridline`) 1) 0 (`KismetArrayLibrary.Array_LastIndex` (`/Game/LumpVR_Basics/Blueprints/VR_ShooterGameMode.GridlinesHorizontal` (`self.GamemodeShort`)))))
        (set `self.GoingDown` false)
        (`self.CWCCW`)))))

(event `CWCCW`
  (bind _speed (`self.Speed`))
  (bind (_currentloc_x _currentloc_y _currentloc_z) (`KismetMathLibrary.BreakVector` (`self.CurrentLoc`)))
  ;[1 1 1] Sideways Clockwise Counterclockwise
  (`self.SetActorHiddenInGame` false)
  (bind (_direction _position) (`Timeline|TimelineEndles` :!via `PlayFromStart` :!label _label)
    (:`Update`
      (set `self.GoingDown` false)
      (if (< _position (* (`KismetMathLibrary.GetPI`) (* (/ 1.0 _speed) 2.0)))
        (bind _returnvalue (+ (`KismetMathLibrary.Atan2` _currentloc_y _currentloc_x) (* _position (* _speed (`self.Direction`)))))
        (bind _outhit (`KismetSystemLibrary.LineTraceSingle` (`KismetMathLibrary.MakeVector` 0.0 0.0 _currentloc_z) (`KismetMathLibrary.MakeVector` (* (`KismetMathLibrary.Cos` _returnvalue) 5000.0) (* (`KismetMathLibrary.Sin` _returnvalue) 5000.0) _currentloc_z) "TraceTypeQuery1"))
        (bind (_bblockinghit _binitialoverlap _time _distance _location _impactpoint _normal _impactnormal _physmat _hitactor) (`GameplayStatics.BreakHitResult` _outhit))
        (if (== (`GameplayStatics.GetObjectClass` _hitactor) "/Game/LumpVR_Basics/Blueprints/BP_Arena01.BP_Arena01_C")
          (bind _position_new (`self.GetActorArenaPos` _location))
          (`self.K2_SetActorTransform` (`KismetMathLibrary.MakeTransform` _position_new (`KismetMathLibrary.ComposeRotators` (`KismetMathLibrary.FindLookAtRotation` (.location (`SceneComponent.K2_GetComponentToWorld` (`self.wurmpart`))) (`KismetMathLibrary.MakeVector` 0.0 0.0 _currentloc_z)) (`KismetMathLibrary.MakeRotator` 0.0 0.0 (* -90 (`self.Direction`)))) (.scale (`SceneComponent.K2_GetComponentToWorld` (`self.wurmpart`))))))
        (else
          (goto _label :!via `PlayFromStart`))))))

(event `StopCWCCW`
  ;[1 1 1] Sideways Clockwise Counterclockwise
  (goto _label :!via `Stop`))

(event `EachXTimer`
  (`KismetSystemLibrary.K2_SetTimer` null "DoEachXTime" (`self.TimerInterval`) true))

(event `DoEachXTime`
  (bind _wurmfront (`self.WurmFront`))
  (if (`self.IAmLeader`)
    ;[1 1 1] Set locations - positions array is pre-filled in event start
    (`KismetArrayLibrary.Array_Set` (`self.Positions`) (`self.PositionIndexCount`) (`self.K2_GetActorLocation` self))
    (set `self.PositionIndexCount` (mod (+ (`self.PositionIndexCount`) 1) (`self.Stored LocationsCount`)))
    (else
      ;[1 1 1] Only deform when frontwurm is present
      (if (not (== _wurmfront null))
        ;[1 1 1] Deform
        (`self.Deform` (`self.wurmpart`) _wurmfront (`KismetMathLibrary.Vector_Distance` (`self.K2_GetActorLocation`) (`self.K2_GetActorLocation` _wurmfront))))
      ;[1 1 1] Get location
      (bind _asbp_wurm (cast `/Game/LumpVR_Basics/Blueprints/BP_Wurm` (`self.MyLead`)))
      (bind _returnvalue (- (`/Game/LumpVR_Basics/Blueprints/BP_Wurm.PositionIndexCount` _asbp_wurm) (* (`self.Wurmnumber`) (`|GetArrayItem` (`/Game/LumpVR_Basics/Blueprints/VR_ShooterGameMode.WurmD_OffsetPerGridline` (`self.GamemodeShort`)) (`/Game/LumpVR_Basics/Blueprints/BP_Wurm.CurrentGridline` _asbp_wurm)))))
      (if (< _returnvalue 0)
        (set `self.PosIndexPositive` (+ _returnvalue (`self.Stored LocationsCount`)))
        (else
          (set `self.PosIndexPositive` _returnvalue)))
      (bind _output (`|GetArrayItem` (`/Game/LumpVR_Basics/Blueprints/BP_Wurm.Positions` _asbp_wurm) (`self.PosIndexPositive`)))
      (if (> (.z _output) 0.0)
        (`self.K2_SetActorTransform` (`KismetMathLibrary.MakeTransform` _output (`self.K2_GetActorRotation` _asbp_wurm)))))))

(event `self.ReceiveTick`
  (params (DeltaSeconds :type "Float (single-precision)")))

(event `self.Sphere.OnComponentBeginOverlap`
  (params (OverlappedComponent :type "PrimitiveComponent Object Reference") (OtherActor :type "Actor Object Reference") (OtherComp :type "PrimitiveComponent Object Reference") (OtherBodyIndex :type Integer) (bFromSweep :type Boolean) (SweepResult :type "HitResult Structure (by ref)"))
  (bind _returnvalue (`GameplayStatics.GetObjectClass` OtherActor))
  (if (`self.SetupDone`)
    (if (== _returnvalue "/Game/LumpVR_Basics/Blueprints/BP_Obstacle.BP_Obstacle_C")
      (if (not (`self.GoingDown`))
        (set `self.GoingDown` true)
        (`self.StopCWCCW`)
        (`self.DDown`))
      (elif (`self.IAmLeader`)
        (if (== _returnvalue "/Game/LumpVR_Basics/Blueprints/BP_Wurm.BP_Wurm_C")
          (if (not (`self.GoingDown`))
            ;[1 1 1] DDown when hitting other wurm
            (bind _asbp_wurm (cast `/Game/LumpVR_Basics/Blueprints/BP_Wurm` OtherActor))
            (if (!= (`/Game/LumpVR_Basics/Blueprints/BP_Wurm.MyLead` _asbp_wurm) (`self.MyLead`))
              (set `self.GoingDown` true)
              (`self.StopCWCCW` _asbp_wurm)
              (`self.DDown` _asbp_wurm))))))))

(event `MakeItLead`
  ;[1 1 1] Make this one Lead
  (set `self.IAmLeader` true)
  (set `self.MyLead` self)
  (set `self.Wurmnumber` 0)
  (`self.SetMaterialAndMesh`)
  (bind _asbp_wurm (cast `/Game/LumpVR_Basics/Blueprints/BP_Wurm` (`self.WurmBehind`)))
  (`self.SetMyLead` _asbp_wurm)
  ;[1 1 1] Sound here because other actors are destroyed
  (`GameplayStatics.PlaySoundAtLocation` "/Game/StarterContent/Audio/Explosion_Cue.Explosion_Cue" (`self.K2_GetActorLocation`) (struct) 1.0 1.0 0.0 null null null))

(event `SetMyLead`
  ;[1 1 1] Make this one follow correct lead
  (`self.SetMaterialandMesh`)
  (bind _asbp_wurm (cast `/Game/LumpVR_Basics/Blueprints/BP_Wurm` (`self.WurmFront`)))
  (set `self.MyLead` (`/Game/LumpVR_Basics/Blueprints/BP_Wurm.MyLead` _asbp_wurm))
  (if (not (`self.IAmLeader`))
    (set `self.Wurmnumber` (+ (`/Game/LumpVR_Basics/Blueprints/BP_Wurm.Wurmnumber` _asbp_wurm) 1))
    (bind _asbp_wurm_2 (cast `/Game/LumpVR_Basics/Blueprints/BP_Wurm` (`self.WurmBehind`)))
    (`self.SetMyLead` _asbp_wurm_2)))

(event `SetMaterialAndMesh`
  (bind _wurmpart (`self.wurmpart`))
  ;[1 1 1] Material and Mesh
  (if (`self.IAmLeader`)
    (`PrimitiveComponent.SetMaterial` _wurmpart 0 "/Game/VirtualReality/Materials/M_ArcEndpoint.M_ArcEndpoint")
    (`StaticMeshComponent.SetStaticMesh` _wurmpart "/Game/StarterContent/Props/MaterialSphere.MaterialSphere")
    (else
      (`PrimitiveComponent.SetMaterial` _wurmpart 0 "/Game/LumpVR_Basics/VFX/MICs/MI_VolumeFlame.MI_VolumeFlame")
      (`StaticMeshComponent.SetStaticMesh` _wurmpart "/Engine/BasicShapes/Sphere.Sphere"))))

(fn `BulletHit`
  (params (HealthAmount :type Integer))
  (bind (_returnvalue_roll _returnvalue_pitch _returnvalue_yaw) (`KismetMathLibrary.BreakRotator` (`KismetMathLibrary.RandomRotator` false)))
  ;[1 1 1] Prevent doubletriggering
  (if (not (`self.HitByBullet`))
    (set `self.HitByBullet` true)
    (set `self.CurrentLoc` (`self.K2_GetActorLocation`))
    (bind _output_get (set `self.Health` (- (`self.Health`) HealthAmount)))
    (if (<= _output_get 0)
      ;[1 1 1] Tell the one behind (if valid) it is the leader
      (bind _wurmbehind (`self.WurmBehind`)
        (:`then`
          (bind _asbp_wurm (cast `/Game/LumpVR_Basics/Blueprints/BP_Wurm` _wurmbehind))
          ;;[1 1 1] Get the current gridline and positions from the leader for DDown
          (bind _asbp_wurm_2 (cast `/Game/LumpVR_Basics/Blueprints/BP_Wurm` (`self.MyLead`)))
          (set `/Game/LumpVR_Basics/Blueprints/BP_Wurm.CurrentGridline` (`/Game/LumpVR_Basics/Blueprints/BP_Wurm.CurrentGridline` _asbp_wurm_2) _asbp_wurm)
          (set `/Game/LumpVR_Basics/Blueprints/BP_Wurm.Positions` (`/Game/LumpVR_Basics/Blueprints/BP_Wurm.Positions` _asbp_wurm_2) _asbp_wurm)
          (set `/Game/LumpVR_Basics/Blueprints/BP_Wurm.PositionIndexCount` (- (- (`/Game/LumpVR_Basics/Blueprints/BP_Wurm.PositionIndexCount` _asbp_wurm_2) 10) (* (`self.Wurmnumber`) (`|GetArrayItem` (`/Game/LumpVR_Basics/Blueprints/VR_ShooterGameMode.WurmD_OffsetPerGridline` (`self.GamemodeShort`)) (`/Game/LumpVR_Basics/Blueprints/BP_Wurm.CurrentGridline` _asbp_wurm_2)))) _asbp_wurm)
          (`self.MakeItLead` _asbp_wurm)
          (`self.StopCWCCW` _asbp_wurm)
          (`self.DDown` _asbp_wurm)
          ;[1 1 1] Comment
          ;;[1 1 1] Spawn Obstacle
          (`|SpawnActorFromClass` "/Game/LumpVR_Basics/Blueprints/BP_Obstacle.BP_Obstacle_C" (`KismetMathLibrary.MakeTransform` (`self.CurrentLoc`) (`KismetMathLibrary.MakeRotator` (`KismetMathLibrary.FClamp` _returnvalue_roll 0.0 10.0) (`KismetMathLibrary.FClamp` _returnvalue_pitch 0.0 10.0) _returnvalue_yaw)) "Undefined" "OverrideRootScale" null null)
          (`self.K2_DestroyActor`))
        (:`else`)))))

(fn `Deform`
  (params (ThisPart :type "StaticMeshComponent Object Reference") (ClosePart :type "Actor Object Reference") (Distance :type "Float (double-precision)"))
  (returns (NewParam :type Boolean))
  (if (== (`GameplayStatics.GetObjectClass` ClosePart) (`GameplayStatics.GetObjectClass` self))
    (bind _returnvalue (`PrimitiveComponent.CreateDynamicMaterialInstance` ThisPart 0 null "NextInLineLoc"))
    (if (> Distance 0.0)
      (`MaterialInstanceDynamic.SetVectorParameterValue` _returnvalue "NextInLineLoc" (`KismetMathLibrary.Conv_VectorToLinearColor` (`self.K2_GetActorLocation` ClosePart)))
      (else
        (`MaterialInstanceDynamic.SetVectorParameterValue` _returnvalue "NextInLineLoc" (struct :`A` 1.0))))
    (else
      (bind _returnvalue_2 (`PrimitiveComponent.CreateDynamicMaterialInstance` ThisPart 0 null "NextInLineLoc"))
      (`MaterialInstanceDynamic.SetVectorParameterValue` :`self` _returnvalue_2 :`ParameterName` "NextInLineLoc"))))

(fn `DEV_PRINTVariableBigorSmall`
  (params (B :type "Float (double-precision)"))
  (if (== (`self.TempCheck`) B)
    (`KismetSystemLibrary.PrintString` "Equal")
    (elif (< B (`self.TempCheck`))
      (`KismetSystemLibrary.PrintString` "Smaller")
      (else
        (`KismetSystemLibrary.PrintString` "Bigger"))))
  (set `self.TempCheck` B))

(fn `GetActorArenaPos`
  (params (`position old` :type "Vector Structure"))
  (returns (`position new` :type "Vector Structure"))
  (bind _x (.x `position old`))
  (bind _y (.y `position old`))
  (bind _z (.z `position old`))
  (bind _returnvalue (`KismetMathLibrary.Atan2` _y _x))
  (bind (_origin _boxextent _sphereradius) (`KismetSystemLibrary.GetComponentBounds` (`self.Sphere`)))
  (bind _outhit (`KismetSystemLibrary.LineTraceSingle` (`KismetMathLibrary.MakeVector` 0.0 0.0 _z) (`KismetMathLibrary.MakeVector` (* _x 5000.0) (* _y 5000.0) _z) "TraceTypeQuery1"))
  (bind (_bblockinghit _binitialoverlap _time _distance _location _impactpoint _normal _impactnormal _physmat _hitactor) (`GameplayStatics.BreakHitResult` _outhit))
  (if (== (`GameplayStatics.GetObjectClass` _hitactor) "/Game/LumpVR_Basics/Blueprints/BP_Arena01.BP_Arena01_C")
    (return (`KismetMathLibrary.MakeVector` (- (.x _location) (/ (* _sphereradius (`KismetMathLibrary.DegSin` (- (- 180.0 (`KismetMathLibrary.RadiansToDegrees` _returnvalue)) 90.0))) (`KismetMathLibrary.DegSin` 90.0))) (- (.y _location) (/ (* _sphereradius (`KismetMathLibrary.DegSin` (`KismetMathLibrary.RadiansToDegrees` _returnvalue))) (`KismetMathLibrary.DegSin` 90.0))) (.z _location)))))

(fn `UserConstructionScript`)