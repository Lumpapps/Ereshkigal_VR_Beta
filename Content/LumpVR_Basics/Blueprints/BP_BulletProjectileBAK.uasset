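; BP_BulletProjectileBAK is a bullet projectile actor that plays a sound and can destroy itself on overlap.
; BeginPlay plays Explosion_Cue at the world origin rather than at the projectile's location.
; When Destructible is set, Box overlaps lead to self-destruction after a cast of the other actor's class and checks excluding BP_Arena01 and itself.
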(event `self.ReceiveBeginPlay`
  (`GameplayStatics.SpawnSoundAtLocation` "/Game/StarterContent/Audio/Explosion_Cue.Explosion_Cue" (0.0 0.0 0.0) (struct) 1.0 1.0 0.0 null null))

(event `self.Box.OnComponentBeginOverlap`
  (params (OverlappedComponent :type "PrimitiveComponent Object Reference") (OtherActor :type "Actor Object Reference") (OtherComp :type "PrimitiveComponent Object Reference") (OtherBodyIndex :type Integer) (bFromSweep :type Boolean) (SweepResult :type "HitResult Structure (by ref)"))
  (if (`self.Destructible`)
    (bind _asactor (castclass `Actor` (`GameplayStatics.GetObjectClass` OtherActor)))
    (if (== _asactor (`GameplayStatics.GetObjectClass` "/Game/LumpVR_Basics/Blueprints/BP_Arena01.BP_Arena01"))
      _
      (elif (not (== OtherActor self))
        (`self.K2_DestroyActor`)))))

(fn `UserConstructionScript`)