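; Actor Blueprint that moves itself back and forth between two fixed target points, switching every two seconds of game time.
; Each Tick selects the target from time modulo four, then lerps from the current location using 25 divided by remaining distance, giving a roughly constant, frame-rate-dependent step.
; Despite the "walkandturn" name, rotation and scale stay unchanged.
; The lerp alpha prints every frame.
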(event `self.ReceiveBeginPlay`
  (set `self.Currentloc` (`self.K2_GetActorLocation`)))

(event `self.ReceiveTick`
  (params (DeltaSeconds :type "Float (single-precision)"))
  (bind (_returnvalue_location _returnvalue_rotation _returnvalue_scale) (`KismetMathLibrary.BreakTransform` (`self.GetTransform`)))
  (bind _goto (`self.GoTo`))
  (bind _returnvalue (/ 25.0 (`KismetMathLibrary.Vector_Distance` _goto _returnvalue_location)))
  (`KismetSystemLibrary.PrintString` (`KismetStringLibrary.Conv_DoubleToString` _returnvalue))
  (if (< (mod (`KismetSystemLibrary.GetGameTimeInSeconds`) 4.0) 2.0)
    (set `self.Currentloc` _returnvalue_location)
    (set `self.GoTo` (`self.0_1000_0`))
    (else
      (set `self.Currentloc` _returnvalue_location)
      (set `self.GoTo` (`self.0_000_0`))))
  (`self.K2_SetActorTransform` (`KismetMathLibrary.MakeTransform` (`KismetMathLibrary.VLerp` (`self.Currentloc`) _goto _returnvalue) _returnvalue_rotation _returnvalue_scale)))

(fn `UserConstructionScript`)