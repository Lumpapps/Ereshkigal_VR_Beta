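; BP_Gridpoint is a grid marker that hands navigation data to a BP_Wurm entering its sphere.
; On overlap, a worm that is not GoingDown receives this point's index as its last gridpoint, plus the plus and minus gridpoint values as locations.
; A Triggered flag gates the overlap and resets only after that handoff, so any other overlap latches the point.
; Gridline data assignments are left unconnected.
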(event `self.ReceiveBeginPlay`)

(event `self.Sphere.OnComponentBeginOverlap`
  (params (OverlappedComponent :type "PrimitiveComponent Object Reference") (OtherActor :type "Actor Object Reference") (OtherComp :type "PrimitiveComponent Object Reference") (OtherBodyIndex :type Integer) (bFromSweep :type Boolean) (SweepResult :type "HitResult Structure (by ref)"))
  (if (not (`self.Triggered`))
    (set `self.Triggered` true)
    (if (== (`GameplayStatics.GetObjectClass` OtherActor) "/Game/LumpVR_Basics/Blueprints/BP_Wurm.BP_Wurm_C")
      (bind _asbp_wurm (cast `/Game/LumpVR_Basics/Blueprints/BP_Wurm` OtherActor))
      (if (not (`/Game/LumpVR_Basics/Blueprints/BP_Wurm.GoingDown` _asbp_wurm))
        (set `/Game/LumpVR_Basics/Blueprints/BP_Wurm.LastGridpointIndex` (`self.GridpointIndex`) _asbp_wurm)
        (set `/Game/LumpVR_Basics/Blueprints/BP_Wurm.PlusLoc` (`self.plusgridpoint`) _asbp_wurm)
        (set `/Game/LumpVR_Basics/Blueprints/BP_Wurm.MinusLoc` (`self.minusgridpoint`) _asbp_wurm)
        (set `self.Triggered` false)))))

(fn `UserConstructionScript`)