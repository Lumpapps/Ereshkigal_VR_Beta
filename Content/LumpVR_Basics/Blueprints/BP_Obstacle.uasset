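; BP_Obstacle is a shootable obstacle that snaps itself to the arena's curved grid.
; On BeginPlay it finds the nearest horizontal gridline from the VR_ShooterGameMode, then rounds its angle down to a cell step derived from that ring's radius and grid size.
; It orients toward a point high above the Arena with randomized roll and pitch.
; BP_BulletProjectile overlaps on its capsule reduce Health until it plays an explosion sound and is destroyed.
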(event `self.ReceiveBeginPlay`
  (bind (_returnvalue_x _returnvalue_y _returnvalue_z) (`KismetMathLibrary.BreakVector` (`self.K2_GetActorLocation`)))
  (bind _indexofclosest (`self.IndexofClosest`))
  ;[1 1 1] Snap to Grid
  (bind _asvr_shooter_game_mode (cast `/Game/LumpVR_Basics/Blueprints/VR_ShooterGameMode` (`GameplayStatics.GetGameMode`)))
  ;;[1 1 1] Find gridnumber by comparing Z to gridlines in stored gridlines Horizontal
  (for (_array_element _array_index) (`/Game/LumpVR_Basics/Blueprints/VR_ShooterGameMode.GridlinesHorizontal` _asvr_shooter_game_mode)
    (if (== _array_index 0)
      (set `self.ClosestGridline` _array_element)
      (bind _returnvalue (`KismetMathLibrary.Abs` (- _array_element _returnvalue_z)))
      (set `self.DistanceToGridline` _returnvalue)
      (set `self.IndexofClosest` _array_index)
      (elif (< _returnvalue (`self.DistanceToGridline`))
        (set `self.ClosestGridline` _array_element)
        (set `self.DistanceToGridline` _returnvalue)
        (set `self.IndexofClosest` _array_index))))
  (bind _asvr_shooter_game_mode_2 (cast `/Game/LumpVR_Basics/Blueprints/VR_ShooterGameMode` (`GameplayStatics.GetGameMode`)))
  (bind _output (`|GetArrayItem` (`/Game/LumpVR_Basics/Blueprints/VR_ShooterGameMode.RadiusAtGridline` _asvr_shooter_game_mode) _indexofclosest))
  (bind _returnvalue_2 (`KismetMathLibrary.Square` _output))
  (bind _gridsize (`/Game/LumpVR_Basics/Blueprints/VR_ShooterGameMode.Gridsize` _asvr_shooter_game_mode))
  (bind _returnvalue_3 (`KismetMathLibrary.Acos` (/ (- (+ _returnvalue_2 _returnvalue_2) (`KismetMathLibrary.Square` _gridsize)) (* (* _output _output) 2.0))))
  (bind _returnvalue_4 (* (`KismetMathLibrary.FFloor` (/ (`KismetMathLibrary.Atan2` _returnvalue_y _returnvalue_x) _returnvalue_3)) _returnvalue_3))
  (bind _returnvalue_5 (`KismetMathLibrary.MakeVector` (* (`KismetMathLibrary.Cos` _returnvalue_4) _output) (* (`KismetMathLibrary.Sin` _returnvalue_4) _output) (+ (`|GetArrayItem` (`/Game/LumpVR_Basics/Blueprints/VR_ShooterGameMode.GridlinesHorizontal` _asvr_shooter_game_mode) _indexofclosest) (* _gridsize 0.5))))
  (bind (_returnvalue_x_2 _returnvalue_y_2 _returnvalue_z_2) (`KismetMathLibrary.BreakVector` (`self.K2_GetActorLocation` (`/Game/LumpVR_Basics/Blueprints/VR_ShooterGameMode.Arena` _asvr_shooter_game_mode_2))))
  (`self.K2_SetActorTransform` (`KismetMathLibrary.MakeTransform` _returnvalue_5 (`KismetMathLibrary.MakeRotator` (+ (.roll (`KismetMathLibrary.FindLookAtRotation` _returnvalue_5 (`KismetMathLibrary.MakeVector` _returnvalue_x_2 _returnvalue_y_2 (+ _returnvalue_z_2 5000.0)))) (- (* (`KismetMathLibrary.RandomFloat`) 10.0) 20.0)) (+ (.pitch (`KismetMathLibrary.FindLookAtRotation` _returnvalue_5 (`KismetMathLibrary.MakeVector` _returnvalue_x_2 _returnvalue_y_2 (+ _returnvalue_z_2 5000.0)))) (- (* (`KismetMathLibrary.RandomFloat`) 10.0) -20.0)) (.yaw (`KismetMathLibrary.FindLookAtRotation` _returnvalue_5 (`KismetMathLibrary.MakeVector` _returnvalue_x_2 _returnvalue_y_2 (+ _returnvalue_z_2 5000.0))))))))

(event `self.Capsule.OnComponentBeginOverlap`
  (params (OverlappedComponent :type "PrimitiveComponent Object Reference") (OtherActor :type "Actor Object Reference") (OtherComp :type "PrimitiveComponent Object Reference") (OtherBodyIndex :type Integer) (bFromSweep :type Boolean) (SweepResult :type "HitResult Structure (by ref)"))
  (if (== (`GameplayStatics.GetObjectClass` OtherActor) "/Game/LumpVR_Basics/Blueprints/BP_BulletProjectile.BP_BulletProjectile_C")
    (bind _output_get (set `self.Health` (- (`self.Health`) 25)))
    (if (<= _output_get 0)
      (`GameplayStatics.SpawnSoundAtLocation` "/Game/StarterContent/Audio/Explosion01.Explosion01" (`self.K2_GetActorLocation`) (struct) 1.0 1.0 0.0 null null)
      (`self.K2_DestroyActor`))))

(fn `UserConstructionScript`)