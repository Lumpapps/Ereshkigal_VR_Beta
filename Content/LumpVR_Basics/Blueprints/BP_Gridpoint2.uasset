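; BP_Gridpoint2 is a path node that steers BP_Wurm and can turn into an obstacle in a VR shooter arena.
; On BeginPlay, about 15% reveal an obstacle mesh, tilted toward a randomized point high on the world's vertical axis.
; On sphere overlap, it passes the worm its neighbor links, choosing the next point by direction.
; Obstacles also start the worm's descent, guarded against retriggering until overlap ends.
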(event `MakeObstacle`
  (set `self.Obstacle` true)
  (`SceneComponent.SetHiddenInGame` (`self.ObstacleMesh`) false false))

(event `self.ReceiveBeginPlay`
  (bind _returnvalue (`self.K2_GetActorLocation`))
  ;[1 1 1] Obstacle or not
  (if (> (`KismetMathLibrary.RandomFloat`) 0.85)
    (`self.MakeObstacle`)
    ;[1 1 1] Random rotation
    (bind _asvr_shooter_game_mode (cast `/Game/LumpVR_Basics/Blueprints/VR_ShooterGameMode` (`GameplayStatics.GetGameMode`)))
    (`self.K2_SetActorTransform` (`KismetMathLibrary.MakeTransform` _returnvalue (`KismetMathLibrary.MakeRotator` (+ (.roll (`KismetMathLibrary.FindLookAtRotation` _returnvalue (`KismetMathLibrary.MakeVector` 0.0 0.0 (* (`/Game/LumpVR_Basics/Blueprints/VR_ShooterGameMode.ArenaHeight` _asvr_shooter_game_mode) (+ (`KismetMathLibrary.RandomFloat`) 2.5))))) (`KismetMathLibrary.NormalizeToRange` (`KismetMathLibrary.RandomFloat`) -10.0 10.0)) (+ (+ (.pitch (`KismetMathLibrary.FindLookAtRotation` _returnvalue (`KismetMathLibrary.MakeVector` 0.0 0.0 (* (`/Game/LumpVR_Basics/Blueprints/VR_ShooterGameMode.ArenaHeight` _asvr_shooter_game_mode) (+ (`KismetMathLibrary.RandomFloat`) 2.5))))) (`KismetMathLibrary.NormalizeToRange` (`KismetMathLibrary.RandomFloat`) -10.0 10.0)) -90.0) (.yaw (`KismetMathLibrary.FindLookAtRotation` _returnvalue (`KismetMathLibrary.MakeVector` 0.0 0.0 (* (`/Game/LumpVR_Basics/Blueprints/VR_ShooterGameMode.ArenaHeight` _asvr_shooter_game_mode) (+ (`KismetMathLibrary.RandomFloat`) 2.5))))))))))

(event `self.Sphere.OnComponentBeginOverlap`
  (params (OverlappedComponent :type "PrimitiveComponent Object Reference") (OtherActor :type "Actor Object Reference") (OtherComp :type "PrimitiveComponent Object Reference") (OtherBodyIndex :type Integer) (bFromSweep :type Boolean) (SweepResult :type "HitResult Structure (by ref)"))
  (if (== (`GameplayStatics.GetObjectClass` OtherActor) "/Game/LumpVR_Basics/Blueprints/BP_Wurm.BP_Wurm_C")
    (bind _asbp_wurm (cast `/Game/LumpVR_Basics/Blueprints/BP_Wurm` OtherActor))
    (set `/Game/LumpVR_Basics/Blueprints/BP_Wurm.LastGridpoint` (`self.K2_GetActorLocation`) _asbp_wurm)
    (set `/Game/LumpVR_Basics/Blueprints/BP_Wurm.BelowLast` (`self.Below`) _asbp_wurm)
    (set `/Game/LumpVR_Basics/Blueprints/BP_Wurm.BelowPlus` (`self.BelowPlus`) _asbp_wurm)
    (set `/Game/LumpVR_Basics/Blueprints/BP_Wurm.BelowMin` (`self.BelowMin`) _asbp_wurm)
    (if (> (`/Game/LumpVR_Basics/Blueprints/BP_Wurm.Direction` _asbp_wurm) 0.0)
      (set `/Game/LumpVR_Basics/Blueprints/BP_Wurm.NextGridpoint` (`self.Plus`) _asbp_wurm)
      (else
        (set `/Game/LumpVR_Basics/Blueprints/BP_Wurm.NextGridpoint` (`self.Minus`) _asbp_wurm)))
    (if (`self.Obstacle`)
      (if (not (`self.OnceYouIdiot`))
        (set `self.OnceYouIdiot` true)
        (if (not (`/Game/LumpVR_Basics/Blueprints/BP_Wurm.GoingDown` _asbp_wurm))
          (`/Game/LumpVR_Basics/Blueprints/BP_Wurm.SetDownLoc` _asbp_wurm)
          (set `/Game/LumpVR_Basics/Blueprints/BP_Wurm.GoingDown` true _asbp_wurm))))))

(event `self.Sphere.OnComponentEndOverlap`
  (params (OverlappedComponent :type "PrimitiveComponent Object Reference") (OtherActor :type "Actor Object Reference") (OtherComp :type "PrimitiveComponent Object Reference") (OtherBodyIndex :type Integer))
  (set `self.OnceYouIdiot` false))

(fn `UserConstructionScript`)