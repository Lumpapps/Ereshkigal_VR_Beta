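; Shootable VR shooter obstacle that sends a BP_Wurm downward when the leader's main collision overlaps its capsule, also counting the down.
; On BeginPlay it tilts toward a randomized point above the world origin, scaled by the game mode's ArenaHeight.
; BulletHit subtracts health and destroys the actor at zero or below.
; A disconnected closest-gridline search for the Wurm never runs.
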(event `self.ReceiveBeginPlay`
  (bind _returnvalue (`self.K2_GetActorLocation`))
  (bind _asvr_shooter_game_mode (cast `/Game/LumpVR_Basics/Blueprints/VR_ShooterGameMode` (`GameplayStatics.GetGameMode`)))
  (`self.K2_SetActorTransform` (`KismetMathLibrary.MakeTransform` _returnvalue (`KismetMathLibrary.MakeRotator` (+ (.roll (`KismetMathLibrary.FindLookAtRotation` _returnvalue (`KismetMathLibrary.MakeVector` 0.0 0.0 (* (`/Game/LumpVR_Basics/Blueprints/VR_ShooterGameMode.ArenaHeight` _asvr_shooter_game_mode) (+ (`KismetMathLibrary.RandomFloat`) 2.5))))) (`KismetMathLibrary.NormalizeToRange` (`KismetMathLibrary.RandomFloat`) -10.0 10.0)) (+ (+ (.pitch (`KismetMathLibrary.FindLookAtRotation` _returnvalue (`KismetMathLibrary.MakeVector` 0.0 0.0 (* (`/Game/LumpVR_Basics/Blueprints/VR_ShooterGameMode.ArenaHeight` _asvr_shooter_game_mode) (+ (`KismetMathLibrary.RandomFloat`) 2.5))))) (`KismetMathLibrary.NormalizeToRange` (`KismetMathLibrary.RandomFloat`) -10.0 10.0)) -90.0) (.yaw (`KismetMathLibrary.FindLookAtRotation` _returnvalue (`KismetMathLibrary.MakeVector` 0.0 0.0 (* (`/Game/LumpVR_Basics/Blueprints/VR_ShooterGameMode.ArenaHeight` _asvr_shooter_game_mode) (+ (`KismetMathLibrary.RandomFloat`) 2.5)))))))))

(event `self.Capsule.OnComponentBeginOverlap`
  (params (OverlappedComponent :type "PrimitiveComponent Object Reference") (OtherActor :type "Actor Object Reference") (OtherComp :type "PrimitiveComponent Object Reference") (OtherBodyIndex :type Integer) (bFromSweep :type Boolean) (SweepResult :type "HitResult Structure (by ref)"))
  ;[1 1 1] Hit by Wurm
  (if (== (`GameplayStatics.GetObjectClass` OtherActor) "/Game/LumpVR_Basics/Blueprints/BP_Wurm.BP_Wurm_C")
    (bind _asbp_wurm (cast `/Game/LumpVR_Basics/Blueprints/BP_Wurm` OtherActor))
    (if (`/Game/LumpVR_Basics/Blueprints/BP_Wurm.IAmLeader` _asbp_wurm)
      (if (== (`/Game/LumpVR_Basics/Blueprints/BP_Wurm.MainCollision` _asbp_wurm) OtherComp)
        (`/Engine/EditorBlueprintResources/StandardMacros.IncrementInt` (`/Game/LumpVR_Basics/Blueprints/BP_Wurm.NumberOfDowns` _asbp_wurm)
          (:`  `
            (set `/Game/LumpVR_Basics/Blueprints/BP_Wurm.GoingDown` true _asbp_wurm)))))))

(fn `BulletHit`
  (params (HealtAmount :type Integer))
  (bind _output_get (set `self.Health` (- (`self.Health`) HealtAmount)))
  (if (<= _output_get 0)
    (`self.K2_DestroyActor`)))

(fn `UserConstructionScript`)